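; Base projectile Blueprint that handles the sound and Niagara effects for a projectile's spawn, flight and impact.
; BeginPlay plays the spawn sound, attaches the flight sound to the root, then spawns muzzle FX facing world X, not the projectile's direction.
; OnSpawnProjectileHitFX plays impact sound and FX at the supplied hit location.
; Muzzle and impact FX spawn only when the flight and impact sounds, respectively, are valid.
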(event EventOnSpawnProjectileHitFX
  (params (HitLocation :type Vector%20%28by%20ref%29 :default "0, 0, 0"))
  (bind _projectileimpactsound (Variables|ProjectileConfig|GetProjectileImpactSound)
    (:then
      (Audio|PlaySoundatLocation _projectileimpactsound HitLocation "0, 0, 0" 1.0 1.0 0.0 0 0 0 0)
      (bind _projectileimpactfx (Variables|ProjectileConfig|GetProjectileImpactFX)
        (:then
          (Niagara|SpawnSystematLocation _projectileimpactfx HitLocation))
        (:else)))
    (:else)))

(event EventBeginPlay
  (bind _returnvalue (Transformation|GetActorLocation))
  (Audio|PlaySoundatLocation (Variables|ProjectileConfig|GetProjectileSpawnSound) _returnvalue "0, 0, 0" 1.0 1.0 0.0 0 0 0 0)
  (bind _projectileflysound (Variables|ProjectileConfig|GetProjectileFlySound)
    (:then
      (Audio|SpawnSoundAttached _projectileflysound (Variables|Transformation|GetRootComponent) "None" "0, 0, 0" "0, 0, 0" "KeepRelativeOffset" true 1.0 1.0 0.0 0 0)
      (bind _projectilemuzzlefx (Variables|ProjectileConfig|GetProjectileMuzzleFX)
        (:then
          (Niagara|SpawnSystematLocation _projectilemuzzlefx _returnvalue (Math|Conversions|RotationFromXVector (Math|Vector|GetForwardVector "0, 0, 0"))))
        (:else)))
    (:else)))

(fn ConstructionScript)