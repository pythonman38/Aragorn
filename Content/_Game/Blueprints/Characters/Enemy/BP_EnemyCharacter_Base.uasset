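; Base enemy character Blueprint that handles the death sequence, dissolving the enemy and its equipped weapon before destroying both.
; OnEnemyDied pauses animation, disables capsule collision, then async-loads and attaches a Niagara effect tinted with the mesh material's dissolve edge color.
; A normalized timeline, rate-scaled by TotalDissolveTime, drives DissolveAmount on both meshes and destroys the actors when finished.
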(event Custom|DisableAnimations
  (Variables|/Script/Engine.SkeletalMeshComponent|SetbPauseAnims (Variables|Character|GetMesh) true)
  (Collision|SetCollisionEnabled (Variables|Default|GetCapsuleComponent) "NoCollision"))

(event Custom|PlayDissolveEffects
  (bind _enemycombatcomponent (Variables|Default|GetEnemyCombatComponent))
  (bind _returnvalue (Class|PawnCombatComponent|GetCharacterCurrentEquippedWeapon _enemycombatcomponent))
  ;[0 0 0] Set a Timer for the Enemy and the Weapon to Dissolve, then Destroy Actors
  (Components|Timeline|SetPlayRate (Variables|Default|GetDissolveTimeline) (/ 1.0 (Variables|Default|GetTotalDissolveTime)))
  (bind _normalizedfloattrack (Timeline|DissolveTimeline PlayFromStart)
    (:Update
      (bind _output_get (Variables|Default|SetNormalizedFloatTrack _normalizedfloattrack))
      (Rendering|Material|SetScalarParameterValueonMaterials (Variables|Character|GetMesh) "DissolveAmount" _output_get)
      (Utilities|IsValid _returnvalue
        (:Is%20Valid
          (Rendering|Material|SetScalarParameterValueonMaterials (Variables|/Script/Aragorn.AragornWeaponBase|GetWeaponMesh _returnvalue) "DissolveAmount" (Variables|Default|GetNormalizedFloatTrack)))))
    (:Finished
      (CallFunction|DestroyActors))))

(event Custom|DestroyActors
  (bind _enemycombatcomponent (Variables|Default|GetEnemyCombatComponent))
  (bind _returnvalue (Class|PawnCombatComponent|GetCharacterCurrentEquippedWeapon _enemycombatcomponent))
  ;[0 0 0] Destroy Enemy and Weapon (if equipped)
  (Utilities|IsValid _returnvalue
    (:Is%20Valid
      (Actor|DestroyActor _returnvalue))
    (:Is%20Not%20Valid
      _))
  (Actor|DestroyActor))

(event Custom|SpawnNiagaraSystem
  (params (Asset :type Object%20Soft%20Object%20Reference))
  (bind _mesh (Variables|Character|GetMesh))
  ;[0 0 0] Play Niaraga Particle System when Enemy Dies
  (bind _object (Utilities|AsyncLoadAsset Asset)
    (:Completed
      (bind _asniagara_system (Utilities|Casting|CastToNiagaraSystem _object))
      (bind _returnvalue (Niagara|SpawnSystemAttached _asniagara_system (Variables|Character|GetMesh) "None" "0, 0, 0" "0, 0, 0" "KeepRelativeOffset" true))
      (bind _returnvalue_2 (Rendering|Material|CreateDynamicMaterialInstance _mesh 0 (Rendering|Material|GetMaterial _mesh 0) "None" :!class /Script/Engine.PrimitiveComponent))
      (bind _returnvalue_3 (Rendering|Material|GetVectorParameterValue _returnvalue_2 "DissolveEdgeColor" :!class /Script/Engine.MaterialInstanceDynamic))
      (Niagara|SetNiagaraVariable(LinearColor) _returnvalue "DissolveParticleColor" _returnvalue_3))))

(event EventBeginPlay)

(event EventOnEnemyDied
  (params (DissolveNiagaraSystem :type Niagara%20System%20Soft%20Object%20Reference))
  (CallFunction|DisableAnimations)
  (CallFunction|SpawnNiagaraSystem DissolveNiagaraSystem)
  (CallFunction|PlayDissolveEffects))

(fn ConstructionScript)