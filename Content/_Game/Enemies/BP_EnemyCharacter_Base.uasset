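; Base enemy character Blueprint that handles the death sequence, dissolving the enemy and its equipped weapon before destroying both.
; On death it pauses animation, disables capsule collision and async-loads a Niagara system attached to the mesh, tinting particles with the material's dissolve edge color.
; A timeline, rate-scaled by the total dissolve time, drives the DissolveAmount parameter on mesh and weapon materials, then destroys both actors when finished.
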(event Custom|SpawnVisualEffects
  (params (Asset :type Object%20Soft%20Object%20Reference))
  (bind _mesh (Variables|Character|GetMesh))
  (Variables|/Script/Engine.SkeletalMeshComponent|SetbPauseAnims (Variables|Character|GetMesh) true)
  (Collision|SetCollisionEnabled (Variables|Default|GetCapsuleComponent) "NoCollision")
  (bind _object (Utilities|AsyncLoadAsset Asset)
    (:Completed
      (bind _asniagara_system (Utilities|Casting|CastToNiagaraSystem _object))
      (bind _returnvalue (Niagara|SpawnSystemAttached _asniagara_system (Variables|Character|GetMesh) "None" "0, 0, 0" "0, 0, 0" "KeepRelativeOffset" true))
      (bind _returnvalue_2 (Rendering|Material|CreateDynamicMaterialInstance _mesh 0 (Rendering|Material|GetMaterial _mesh 0) "None" :!class /Script/Engine.PrimitiveComponent))
      (bind _returnvalue_3 (Rendering|Material|GetVectorParameterValue _returnvalue_2 "DissolveEdgeColor" :!class /Script/Engine.MaterialInstanceDynamic))
      (Niagara|SetNiagaraVariable(LinearColor) _returnvalue "DissolveParticleColor" _returnvalue_3))))

(event Custom|PlayDissolveEffects
  (bind _enemycombatcomponent (Variables|Default|GetEnemyCombatComponent))
  (bind _returnvalue (Class|PawnCombatComponent|GetCharacterCurrentEquippedWeapon _enemycombatcomponent))
  (Components|Timeline|SetPlayRate (Variables|Default|GetDissolveTimeline) (/ 1.0 (Variables|Default|GetTotalDissolveTime)))
  (bind _normalizedfloattrack (Timeline|DissolveTimeline PlayFromStart)
    (:Update
      (bind _output_get (Variables|Default|SetFloatTrackValue _normalizedfloattrack))
      (Rendering|Material|SetScalarParameterValueonMaterials (Variables|/Script/Aragorn.AragornWeaponBase|GetWeaponMesh _returnvalue) "DissolveAmount" _output_get)
      (Rendering|Material|SetScalarParameterValueonMaterials (Variables|Character|GetMesh) "DissolveAmount" (Variables|Default|GetFloatTrackValue)))
    (:Finished
      (Utilities|IsValid _returnvalue
        (:Is%20Valid
          (Actor|DestroyActor _returnvalue))
        (:Is%20Not%20Valid
          _))
      (Actor|DestroyActor))))

(event EventBeginPlay)

(event Collision|EventActorBeginOverlap
  (params (OtherActor :type Actor%20Object%20Reference)))

(event EventTick
  (params (DeltaSeconds :type Float%20%28single-precision%29)))

(event EventOnEnemyDied
  (params (DissolveNiagaraSystem :type Niagara%20System%20Soft%20Object%20Reference))
  (CallFunction|SpawnVisualEffects DissolveNiagaraSystem)
  (CallFunction|PlayDissolveEffects))

(fn ConstructionScript)